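; BP_EA_CircularLabyrinth is an unfinished actor Blueprint, apparently intended to generate a circular labyrinth from splines.
; Its Generate event calls FirstCircle, which adds a spline component and a single point with no computed position.
; Unconnected trig nodes using Divisions and SectorSize, plus an unreached AddPoints call, suggest planned ring placement that is not yet wired.
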(event `Generate`
  (`self.FirstCircle`))

(fn `FirstCircle`
  (bind _returnvalue (`AddComponent|NODE_AddSplineComponent-0`))
  (`SplineComponent.AddPoint` _returnvalue (make `SplinePoint` 0.0) true))

(fn `UserConstructionScript`)