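; Dead-end floor piece for the labyrinth, built procedurally in the construction script as a grid of stone tiles and tagged Bp_Floor.
; Tile size and count derive from the floor size, mesh bounds and tiles per section, with an optional centred pivot.
; Tiles are brown-material HISM instances, given seeded random height offsets and optional random rotation from a stream.
; The event graph has no runtime logic.
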(fn `UserConstructionScript`
  (locals (L_StoneSizeX :type "Float (double-precision)") (L_StoneSizeY :type "Float (double-precision)") (L_StoneLocation :type "Vector Structure" :default (0.0 0.0 0.0)) (L_StoneRotation :type "Rotator Structure" :default (struct)) (L_StoneScale :type "Vector Structure" :default (1.0 1.0 1.0)) (L_StoneLocation_X :type "Vector Structure") (L_StoneLocation_Y :type "Vector Structure") (L_X :type Integer :default 1) (L_Y :type Integer :default 1))
  (bind _maxrndrotfloor (`self.MaxRndRotFloor`))
  (bind _l_stonelocation (`local.L_StoneLocation`))
  (bind (_returnvalue_min _returnvalue_max) (break `Box` (`StaticMesh.GetBoundingBox` (`self.SM_Floor`))))
  (bind (_returnvalue_min_2 _returnvalue_max_2) (break `Box` (`StaticMesh.GetBoundingBox` (`self.SM_Floor`))))
  (bind _returnvalue (* (`self.MaxRndRotFloor`) -1.0))
  (bind _returnvalue_2 (/ (`KismetMathLibrary.Conv_IntToDouble` (`self.FloorSizeXY`)) 2.0))
  (bind _returnvalue_x (`KismetMathLibrary.BreakVector` (- _returnvalue_max_2 _returnvalue_min_2)))
  (bind (_returnvalue_x_2 _returnvalue_y) (`KismetMathLibrary.BreakVector` (- _returnvalue_max _returnvalue_min)))
  (`KismetArrayLibrary.Array_Clear` (`self.Tags`))
  (`KismetArrayLibrary.Array_AddUnique` (`self.Tags`) "Bp_Floor")
  (if (and (> (`self.FloorSizeXY`) 0) (`KismetSystemLibrary.IsValid` (`self.SM_Floor`)))
    (`StaticMeshComponent.SetStaticMesh` (`self.HISM_00`) (`self.SM_Floor`))
    (`PrimitiveComponent.SetMaterial` (`self.HISM_00`) 0 "/Game/LabyrinthS/Materials/MI_Brown.MI_Brown")
    (set `local.L_StoneSizeX` (* (/ (`KismetMathLibrary.Conv_IntToDouble` (`self.FloorSizeXY`)) _returnvalue_x) (/ 100.0 (`self.TilesPerFloorSection`))))
    (set `local.L_StoneSizeY` (* (/ (`KismetMathLibrary.Conv_IntToDouble` (`self.FloorSizeXY`)) _returnvalue_y) (/ 100.0 (`self.TilesPerFloorSection`))))
    (set `local.L_X` (`KismetMathLibrary.Round` (/ (`self.FloorSizeXY`) (`local.L_StoneSizeX`))))
    (set `local.L_Y` (`KismetMathLibrary.Round` (/ (`self.FloorSizeXY`) (`local.L_StoneSizeY`))))
    (for _index (range (`local.L_X`))
      (set `local.L_StoneLocation_X` (+ (* _index (`KismetMathLibrary.MakeVector` (`local.L_StoneSizeX`))) (`KismetMathLibrary.MakeVector` 0.0 0.0 (`self.StoneZOffset`))))
      (for _index_2 (range (`local.L_Y`))
        (set `local.L_StoneLocation_Y` (* _index_2 (`KismetMathLibrary.MakeVector` 0.0 (`local.L_StoneSizeY`))))
        (set `local.L_StoneLocation` (+ (`local.L_StoneLocation_X`) (`local.L_StoneLocation_Y`)))
        (`InstancedStaticMeshComponent.AddInstance` (`self.HISM_00`) (`KismetMathLibrary.MakeTransform` (+ (select `bool` (`self.bCenterPivot`) :`false` _l_stonelocation :`true` (- _l_stonelocation (`KismetMathLibrary.MakeVector` _returnvalue_2 _returnvalue_2))) (`KismetMathLibrary.MakeVector` 0.0 0.0 (`KismetMathLibrary.RandomFloatInRangeFromStream` (`self.Stream`) (`self.MinZOffser`) (`self.MaxZOffset`)))) (select `bool` (`self.bRndRotation`) :`false` (`local.L_StoneRotation`) :`true` (`KismetMathLibrary.MakeRotator` (`KismetMathLibrary.RandomFloatInRangeFromStream` (`self.Stream`) _returnvalue _maxrndrotfloor) (`KismetMathLibrary.RandomFloatInRangeFromStream` (`self.Stream`) _returnvalue _maxrndrotfloor) (`KismetMathLibrary.RandomFloatInRangeFromStream` (`self.Stream`) _returnvalue _maxrndrotfloor))) (`KismetMathLibrary.MakeVector` (/ (`local.L_StoneSizeX`) 100.0) (/ (`local.L_StoneSizeY`) 100.0) (`self.StoneScaleZ`))) false)))))